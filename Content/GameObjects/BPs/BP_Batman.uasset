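; BP_Batman is a movable Batman actor that shifts left and right along the Y axis.
; MoveLeft and MoveRight call the parent handlers, then restart a shared Move timeline if IsMoving is set.
; The timeline lerps Y from the actor's current location toward TargetLocation, keeping X and Z, and clears the moving state when finished.
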(event EventBeginPlay)

(event Collision|EventActorBeginOverlap
  (params (OtherActor :type Actor%20Object%20Reference)))

(event EventTick
  (params (DeltaSeconds :type Float%20%28single-precision%29)))

(event EventMoveLeft
  (params (Value :type Input%20Action%20Value%20Structure%20%28by%20ref%29))
  (bind _returnvalue (Transformation|GetActorLocation))
  (|CallParentFunction Value)
  (if (Variables|Default|GetbIsMoving)
    (bind _move (Timeline|Move PlayFromStart)
      (:Update
        (Transformation|SetActorLocation (Math|Vector|MakeVector (.x _returnvalue) (Math|Float|Lerp (.y _returnvalue) (Variables|Default|GetTargetLocation) _move) (.z _returnvalue)) false false))
      (:Finished
        (Class|Batman|SetMoving false)))))

(event EventMoveRight
  (params (Value :type Input%20Action%20Value%20Structure%20%28by%20ref%29))
  (bind _returnvalue (Transformation|GetActorLocation))
  (|CallParentFunction Value)
  (if (Variables|Default|GetbIsMoving)
    (bind _move (Timeline|Move PlayFromStart)
      (:Update
        (Transformation|SetActorLocation (Math|Vector|MakeVector (.x _returnvalue) (Math|Float|Lerp (.y _returnvalue) (Variables|Default|GetTargetLocation) _move) (.z _returnvalue)) false false))
      (:Finished
        (Class|Batman|SetMoving false)))))

(fn ConstructionScript)